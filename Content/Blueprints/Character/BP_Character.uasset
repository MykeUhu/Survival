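; BP_Character is a character Blueprint that prints debug readouts of total distance walked and run in kilometres every tick.
; The distance getters are called but not defined in its graphs.
; Tick also passes the Movement.Speed.2 gameplay tag to TestCheckTags, an empty test function with an unconnected HasAnyTags check.
; BeginPlay, ActorBeginOverlap and the construction script are empty.
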(event EventBeginPlay)

(event Collision|EventActorBeginOverlap
  (params (OtherActor :type Actor%20Object%20Reference)))

(event EventTick
  (params (DeltaSeconds :type Float%20%28single-precision%29))
  (CallFunction|TestCheckTags "(GameplayTags=((TagName=\"Movement.Speed.2\")))")
  (Development|PrintString (Utilities|String|ToString(Float) (Class|UhuSurvivalCharacter|GetTotalDistanceWalkedKM)))
  (Development|PrintString (Utilities|String|ToString(Float) (Class|UhuSurvivalCharacter|GetTotalDistanceRunKM))))

(fn ConstructionScript)

(fn TestCheckTags
  (params (GameplayTagContainer :type Gameplay%20Tag%20Container%20Structure)))